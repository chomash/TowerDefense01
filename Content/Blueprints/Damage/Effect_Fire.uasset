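; Fire damage-over-time effect that periodically damages its owning actor.
; Tick runs through a Delay of TickInterval, so damage is applied at intervals using Damage_Basic, with the result printed for debugging.
; ApplyEffect sets the damage to TickDamage, and RefreshEffect adds another TickDamage per stack up to MaxStackSize when the effect is stackable.
; It extends a parent effect, calling its Tick, apply and refresh logic first.
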(event EventBeginPlay
  (|CallParentFunction) ; This node is disabled and will not be called.\nDrag off pins to build functionality.
)

(event EventTick
  (params (DeltaSeconds :type Float%20%28single-precision%29))
  (Utilities|FlowControl|Sequence
    (:then_0
      (|CallParentFunction DeltaSeconds))
    (:then_1
      (Utilities|FlowControl|Delay (Variables|Default|GetTickInterval))
      (bind _returnvalue (Game|Damage|ApplyDamage (Variables|Default|GetOwningActor) (Variables|Default|GetFinalDamage) 0 0 "/Game/Blueprints/Damage/Damage_Basic.Damage_Basic_C"))
      (Development|PrintString (Utilities|String|ToString(Float) _returnvalue)))))

(event EventRefreshEffect
  (|CallParentFunction)
  (if (and (Variables|Default|GetStackable) (< (Variables|Default|GetStackSize) (Variables|Default|GetMaxStackSize)))
    (Math|Integer|IncrementInt (Variables|Default|GetStackSize)
      (:%20%20
        (Variables|Default|SetFinalDamage (+ (Variables|Default|GetFinalDamage) (Variables|Default|GetTickDamage)))))))

(event EventApplyEffect
  (|CallParentFunction)
  (Variables|Default|SetFinalDamage (Variables|Default|GetTickDamage)))