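; Timed effect component for BP_EnemyBasic actors, providing apply, refresh and remove events for an effect with a limited duration.
; On BeginPlay it stores the owning enemy and applies itself, setting a finish time from current game time plus Duration.
; RefreshEffect restarts that duration only when the effect is Refreshable.
; Tick compares game time to the finish time and destroys the component through RemoveEffect on expiry.
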(event Custom|ApplyEffect
  (Utilities|CalculateFinishTime))

(event Custom|RefreshEffect
  (if (Variables|Default|GetRefreshable)
    (Utilities|CalculateFinishTime)))

(event Custom|RemoveEffect
  (Components|DestroyComponent))

(event EventBeginPlay
  (bind _asbp_enemy_basic (Utilities|Casting|CastToBP_EnemyBasic (Components|GetOwner)))
  (Variables|Default|SetOwningActor _asbp_enemy_basic)
  (CallFunction|ApplyEffect))

(event EventTick
  (params (DeltaSeconds :type Float%20%28single-precision%29))
  (if (>= (Utilities|Time|GetGameTimeinSeconds) (Variables|Default|GetFinishTime))
    (CallFunction|RemoveEffect)))