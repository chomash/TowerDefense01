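; Electro damage effect component that has a chance to stun its owning actor by stopping its movement.
; On apply, a check requires the owner to be neither stun immune nor just stunned and to pass a weighted random roll, otherwise the component destroys itself.
; A successful stun saves and zeroes walk speed and sets stun immunity.
; Removal restores the saved speed but leaves immunity untouched.
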(event EventBeginPlay
  (|CallParentFunction))

(event EventTick
  (params (DeltaSeconds :type Float%20%28single-precision%29))
  (|CallParentFunction DeltaSeconds))

(event EventApplyEffect
  (bind _owningactor (Variables|Default|GetOwningActor))
  (bind _charactermovement (Variables|/Script/Engine.Character|GetCharacterMovement _owningactor))
  (Utilities|CheckStunCondition
    (:CanStun
      (Variables|Default|SetDefaultSpeed (Variables|/Script/Engine.CharacterMovementComponent|GetMaxWalkSpeed _charactermovement))
      (Variables|/Script/Engine.CharacterMovementComponent|SetMaxWalkSpeed _charactermovement 0.0)
      (Default|SetStunImmune (Variables|Default|GetOwningActor) true)
      (|CallParentFunction))
    (:Can'tStun
      (Components|DestroyComponent))))

(event EventRemoveEffect
  (Variables|/Script/Engine.CharacterMovementComponent|SetMaxWalkSpeed (Variables|/Script/Engine.Character|GetCharacterMovement (Variables|Default|GetOwningActor)) (Variables|Default|GetDefaultSpeed))
  (|CallParentFunction))