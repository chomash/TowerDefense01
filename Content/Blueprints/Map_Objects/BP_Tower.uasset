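; BP_Tower is a map object with health that enemies damage on contact, ending the game when its health runs out.
; An enemy overlapping its box passes its damage info to TakeDamage and is destroyed.
; TakeDamage clamps TowerHealth, updates the HUD health widget and calls GameOver at zero, which only prints a message.
; Heal and both health getters are stubs returning zero.
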(event OnComponentBeginOverlap(Box)
  (params (OverlappedComponent :type Primitive%20Component%20Object%20Reference) (OtherActor :type Actor%20Object%20Reference) (OtherComp :type Primitive%20Component%20Object%20Reference) (OtherBodyIndex :type Integer) (bFromSweep :type Boolean) (SweepResult :type Hit%20Result%20Structure%20%28by%20ref%29))
  (bind _as_bp_enemy_base (Utilities|Casting|CastTo_BP_EnemyBase OtherActor))
  (CallFunction|TakeDamage (Variables|/Game/Blueprints/Enemy/_BP_EnemyBase._BP_EnemyBase_C|GetDamage%20Info _as_bp_enemy_base))
  (Actor|DestroyActor _as_bp_enemy_base))

(event EventBeginPlay
  (Utilities|FlowControl|Delay 0.0)
  (Class|BPIHUD|UpdateHealthWidget(Message) (HUD|GetHUD (Game|GetPlayerController 0)) (Variables|Default|GetTowerHealth)))

(fn ConstructionScript)

(fn GameOver
  (Development|PrintString "GAME OVER"))

(fn GetCurrentHealth
  (return 0.0))

(fn GetMaxHealth
  (return 0.0))

(fn Heal
  (params (Amount :type Float%20%28double-precision%29))
  (return 0.0))

(fn TakeDamage
  (params (DamageInf :type S%20Damage%20Info%20Structure))
  (bind _output_get (Variables|Default|SetTowerHealth (Math|Float|Clamp(Float) (- (Variables|Default|GetTowerHealth) (.amount DamageInf)) 0.0 2e+05)))
  (Class|BPIHUD|UpdateHealthWidget(Message) (HUD|GetHUD (Game|GetPlayerController 0)) _output_get)
  (if (> _output_get 0.0)
    (return true)
    (else
      (CallFunction|GameOver)
      (return true))))