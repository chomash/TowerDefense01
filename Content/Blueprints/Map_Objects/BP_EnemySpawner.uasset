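; Enemy spawner map object that runs waves of AI enemies from the moment play begins.
; It reads each wave in row order from a data table, then spawns its chunks of one enemy type each.
; Nested macro loops apply separate delays between enemies, chunks and waves.
; Each enemy spawns at the Arrow component's location and rotation and is initialized with the spline path.
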(event Custom|SpawnNextWave
  (if (Variables|WaveControl|GetCanSpawnNextWave)
    (CallFunction|GetNewWaveInfo)
    (Utilities|SpawnNewWave
      (:Completed
        (Utilities|FlowControl|Delay (Variables|WaveControl|GetSpawnDelay_Wave))
        (CallFunction|SpawnNextWave)))))

(event EventBeginPlay
  (CallFunction|SpawnNextWave))

(fn ConstructionScript)

(fn SpawnEnemy
  (params (EnemyToSpawn :type BP%20Enemy%20Base%20Class%20Reference))
  (bind _arrow (Variables|Default|GetArrow))
  (bind _returnvalue (AI|SpawnAIFromClass EnemyToSpawn 0 (Transformation|GetWorldLocation _arrow) (Transformation|GetWorldRotation _arrow) false 0))
  (bind _as_bp_enemy_base (Utilities|Casting|CastTo_BP_EnemyBase _returnvalue))
  (Default|Initialize _as_bp_enemy_base (Variables|Default|GetSplinePath)))

(fn GetNewWaveInfo
  (bind _wave_dt (Variables|WaveControl|GetWave_DT))
  (bind _outrownames (DataTable|GetDataTableRowNames _wave_dt))
  (bind _returnvalue (Utilities|GetDataTableRow _wave_dt (Utilities|Array|Get(acopy) _outrownames (Variables|WaveControl|GetWaveNumber)))
    (:then
      (Variables|WaveControl|SetCurrentWave _returnvalue)
      (bind _result (Math|Integer|IncrementInt (Variables|WaveControl|GetWaveNumber))
        (:%20%20
          (Variables|WaveControl|SetCanSpawnNextWave (< _result (Utilities|Array|Length _outrownames))))))))