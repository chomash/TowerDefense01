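; BP_Turret_Projectile is a defense turret that fires a short burst of projectiles.
; On Fire, it runs the parent logic, then spawns BP_Projectile at the WeaponBallistaArrow transform, passing itself as owner along with its DamageInfo.
; A DoN node, reset on each Fire, loops back through a short Delay to produce a two-shot burst.
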(event EventBeginPlay
  (|CallParentFunction))

(event Collision|EventActorBeginOverlap
  (params (OtherActor :type Actor%20Object%20Reference))
  (|CallParentFunction OtherActor) ; This node is disabled and will not be called.\nDrag off pins to build functionality.
)

(event EventTick
  (params (DeltaSeconds :type Float%20%28single-precision%29))
  (|CallParentFunction DeltaSeconds) ; This node is disabled and will not be called.\nDrag off pins to build functionality.
)

(event EventFire
  (|CallParentFunction)
  (Utilities|FlowControl|Sequence
    (:then_0
      (goto _label Reset))
    (:then_1
      (Utilities|FlowControl|DoN 2 :!label _label
        (:Exit
          (Game|SpawnActorfromClass "/Game/Blueprints/Map_Objects/Defense/BP_Projectile.BP_Projectile_C" (Transformation|GetWorldTransform (Variables|Default|Getweapon_ballista_arrow)) "Undefined" "MultiplyWithRoot" self (Variables|Default|GetDamageInfo) 0)
          (Utilities|FlowControl|Delay 0.2)
          (goto _label))))))

(fn ConstructionScript
  (|CallParentFunction))