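; Enemy AI controller that runs its pawn along a referenced spline path when RunAlongSpline is triggered.
; It derives the run duration from spline length and the owner's max speed, then scales a timeline's play rate by its inverse.
; Each timeline update maps alpha to a distance along the spline and issues MoveToLocation to that world point with pathfinding disabled.
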(event Custom|RunAlongSpline
  (CallFunction|CalculateRunDuration)
  (Components|Timeline|SetPlayRate (Variables|Default|GetMoveTimeline) (/ 1.0 (Variables|Default|GetRunDuration)))
  (bind _alpha (Timeline|MoveTimeline Play)
    (:Update
      (Variables|Default|SetAlpha _alpha)
      (AI|Navigation|MovetoLocation (Spline|GetLocationatDistanceAlongSpline (Variables|/Game/Blueprints/Enemy/BP_Spline.BP_Spline_C|GetSplinePath (Variables|Default|GetSplineReference)) (Math|Float|Lerp 0.0 (Spline|GetSplineLength (Variables|/Game/Blueprints/Enemy/BP_Spline.BP_Spline_C|GetSplinePath (Variables|Default|GetSplineReference))) (Variables|Default|GetAlpha)) "World") -1.0 true false false true 0))))

(fn ConstructionScript)

(fn CalculateRunDuration
  (Variables|Default|SetRunDuration (/ (Spline|GetSplineLength (Variables|/Game/Blueprints/Enemy/BP_Spline.BP_Spline_C|GetSplinePath (Variables|Default|GetSplineReference))) (Variables|Default|GetOwnerMaxSpeed))))