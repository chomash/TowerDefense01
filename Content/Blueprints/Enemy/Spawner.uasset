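; Enemy spawner actor that spawns BP_EnemyBasic AI at its own transform and sends them along a list of target points.
; On BeginPlay, a delayed loop spawns until the configured count is reached, passing each enemy the points and starting its run.
; The construction script calls DrawDebugLines to preview the route with temporary debug lines from the spawner through the target points.
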(event EventBeginPlay
  (bind _self self)
  (bind _defaultsceneroot (Variables|Default|GetDefaultSceneRoot _self))
  (if (< (Variables|Default|GetSpawnCount) (Variables|Default|GetEnemiesToSpawnCount)) :!label _label
    (bind _returnvalue (AI|SpawnAIFromClass "/Game/Blueprints/Enemy/BP_EnemyBasic.BP_EnemyBasic_C" 0 (Transformation|GetWorldLocation _defaultsceneroot) (Transformation|GetWorldRotation _defaultsceneroot) false 0))
    (bind _asbp_enemy_basic (Utilities|Casting|CastToBP_EnemyBasic _returnvalue))
    (Variables|/Game/Blueprints/Enemy/BP_EnemyBasic.BP_EnemyBasic_C|SetPoints%20to%20Move _asbp_enemy_basic (Variables|Default|GetTargetPoints))
    (Default|RunBabyRun _asbp_enemy_basic)
    (Math|Integer|IncrementInt (Variables|Default|GetSpawnCount)
      (:%20%20
        (Utilities|FlowControl|Delay (Variables|Default|GetSpawnDelay))
        (goto _label)))))

(fn ConstructionScript
  (Utilities|DrawDebugLines))