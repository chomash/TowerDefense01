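; Basic enemy that follows a supplied list of points via AI MoveTo and destroys itself at the end of the path.
; Damage is scaled by per-type resistance, updates a health bar widget and destroys the enemy at zero health.
; Each damage type's class defaults name an effect component, which is added on hit or refreshed if already present.
; Tick clears a timed stun-immunity flag.
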(event Custom|RunBabyRun
  (bind _points_to_move (Variables|POI|GetPoints%20to%20Move))
  (bind _asenemy_ai_controller (Utilities|Casting|CastToEnemyAiController (Pawn|GetController)))
  (Variables|Components|SetAIController _asenemy_ai_controller)
  (bind _output_get (Variables|POI|SetLastIndexToMove (Utilities|Array|Length _points_to_move)))
  (if (not (== _output_get (Variables|POI|GetLocationIndex))) :!label _label
    (AI|AIMoveTo (Variables|Components|GetAIController) "0, 0, 0" (Utilities|Array|Get(acopy) _points_to_move (Variables|POI|GetLocationIndex)) 1e+02 "Default" "Default" true true
      (:OnMoveFinished
        (bind _result (Math|Integer|IncrementInt (Variables|POI|GetLocationIndex))
          (:%20%20
            (Variables|POI|SetLocationIndex _result)
            (goto _label)))))
    (else
      (Actor|DestroyActor))))

(event Custom|SetStunImmune
  (params (Immune :type Boolean))
  (bind _output_get (Variables|Defenses|SetJustStunned Immune))
  (if _output_get
    (Variables|Defenses|SetStunImmuneFinishTime (+ (Utilities|Time|GetGameTimeinSeconds) (Variables|Defenses|GetStunImmuneDuration)))))

(event EventBeginPlay
  (Variables|Components|SetAs%20WB%20HP (.AsWB%20HP (Utilities|Casting|CastToWB_HP (UserInterface|GetWidget (Variables|Default|GetWidget)))))
  (Variables|Default|SetCurrentHealth (Variables|Default|GetMaxHealth))
  (Default|UpdateHealthWidget (Variables|Components|GetAs%20WB%20HP) (Utilities|GetHealthPer)))

(event Game|Damage|EventAnyDamage
  (params (Damage :type Float%20%28single-precision%29) (DamageType :type Damage%20Type%20Object%20Reference) (InstigatedBy :type Controller%20Object%20Reference) (DamageCauser :type Actor%20Object%20Reference))
  (bind _finaldamage (CallFunction|DamageCalculation Damage DamageType))
  (CallFunction|AddEffect DamageType)
  (bind _output_get (Variables|Default|SetCurrentHealth (- (Variables|Default|GetCurrentHealth) _finaldamage)))
  (if (<= _output_get 0.0)
    (Actor|DestroyActor)
    (else
      (Default|UpdateHealthWidget (Variables|Components|GetAs%20WB%20HP) (Utilities|GetHealthPer)))))

(event EventTick
  (params (DeltaSeconds :type Float%20%28single-precision%29))
  (Utilities|CheckStunImmuneStatus))

(fn ConstructionScript)

(fn Initialize
  (params (PointsToMove :type Array%20of%20Actor%20Object%20References))
  (Variables|POI|SetPoints%20to%20Move PointsToMove))

(fn DamageCalculation
  (params (InitialDamage :type Float%20%28double-precision%29) (DamageType :type Damage%20Type%20Object%20Reference))
  (return (* InitialDamage (.Value (Utilities|Map|Find (Variables|Defenses|GetDamageResistance) (.As%20Damage%20Type (Utilities|Casting|CastTo_DamageTypeClass (Utilities|GetClass DamageType))))))))

(fn AddEffect
  (params (DamageType :type Damage%20Type%20Object%20Reference))
  (bind _as_damage_type (Utilities|Casting|CastTo_DamageTypeClass (Utilities|GetClass DamageType))
    (:then
      (if (== (Utilities|Array|Length (Actor|GetComponentsByClass (Utilities|GetClassDefaults _as_damage_type))) 0)
        (Game|AddComponentbyClass (Utilities|GetClassDefaults _as_damage_type))
        (return)
        (else
          (for _array_element (Actor|GetComponentsByClass (Utilities|GetClassDefaults _as_damage_type))
            (Default|RefreshEffect _array_element)
            (return)))))
    (:CastFailed
      (return))))