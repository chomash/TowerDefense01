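; Tower defense game mode that holds the player's coin balance and keeps the HUD coin display in sync with it.
; Adding or removing coins updates the total, with removal clamped at zero, and passes the new value to the player HUD through UpdateCoinWidgetMessage.
; On BeginPlay it adds one coin after a zero-length delay, which also triggers the first HUD refresh.
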(event EventBeginPlay
  (Utilities|FlowControl|Delay 0.0)
  (LevelState|AddCoins 1))

(fn ConstructionScript)

(fn AddCoins
  (params (Amount :type Integer))
  (bind _output_get (Variables|LevelState|SetCoins (+ Amount (Variables|LevelState|GetCoins))))
  (Utilities|UpdateCoinWidget _output_get)
  (return _output_get))

(fn RemoveCoins
  (params (Amount :type Integer))
  (bind _output_get (Variables|LevelState|SetCoins (Math|Integer|Clamp(Integer) (- (Variables|LevelState|GetCoins) Amount) 0 2147483647)))
  (Utilities|UpdateCoinWidget _output_get)
  (return _output_get))